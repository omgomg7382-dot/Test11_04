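; BP_GM is a stage-flow manager that handles clearing a stage and moving to the next level.
; Its GameReStart event queries actors by tag, with the tag set to None, and treats an empty result as a clear.
; On a clear it prints a message, waits briefly, then opens the level named by the 다음판 (next stage) variable on the first BP_StageName actor found.
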(event `Game ReStart`
  (bind _outactors (`GameplayStatics.GetAllActorsWithTag` "None"))
  (if (== (`KismetArrayLibrary.Array_Length` _outactors) 0)
    (`KismetSystemLibrary.PrintString` "Clear! Next Stage")
    (`KismetSystemLibrary.Delay` 3.0)
    (bind _outactors_2 (`GameplayStatics.GetAllActorsOfClass` "/Game/BluePrint/BP_StageName.BP_StageName_C"))
    (`GameplayStatics.OpenLevel` (`KismetStringLibrary.Conv_StringToName` (`/Game/BluePrint/BP_StageName.다음판` (`|GetArrayItem` _outactors_2))))))

(fn `UserConstructionScript`)