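; BP_Rocket is a rocket projectile that destroys itself three seconds after it begins play.
; When it overlaps an actor tagged Target, it destroys that actor and plays an explosion sound and enlarged particle effect at its own location.
; It then casts the game mode to BP_GM, calls GameReStart and destroys itself.
; The Box overlap event is empty.
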(event `self.ReceiveBeginPlay`
  (`KismetSystemLibrary.Delay` 3.0)
  (`self.K2_DestroyActor`))

(event `self.ReceiveActorBeginOverlap`
  (params (OtherActor :type "Actor Object Reference"))
  (if (`self.ActorHasTag` OtherActor "Target")
    (`self.K2_DestroyActor` OtherActor)
    (`GameplayStatics.SpawnSoundAtLocation` "/Game/StarterContent/Audio/Explosion_Cue.Explosion_Cue" (`self.K2_GetActorLocation`) (struct) 1.0 1.0 0.0 null null)
    (`GameplayStatics.SpawnEmitterAtLocation` "/Game/StarterContent/Particles/P_Explosion.P_Explosion" (`self.K2_GetActorLocation`) (struct) (2.0 2.0 2.0))
    (bind _asbp_gm (cast `/Game/BluePrint/BP_GM` (`GameplayStatics.GetGameMode`)))
    (`/Game/BluePrint/BP_GM.Game ReStart` _asbp_gm)
    (`self.K2_DestroyActor`)))

(event `self.Box.OnComponentBeginOverlap`
  (params (OverlappedComponent :type "PrimitiveComponent Object Reference") (OtherActor :type "Actor Object Reference") (OtherComp :type "PrimitiveComponent Object Reference") (OtherBodyIndex :type Integer) (bFromSweep :type Boolean) (SweepResult :type "HitResult Structure (by ref)")))

(fn `UserConstructionScript`)