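; BP_P38_Main is a player-controlled P-38 plane that flies continuously forward and fires rockets.
; Tick feeds constant forward movement input and spins both propellers through RotateComponent, scaled by delta time.
; Pitch and Roll axes rotate the actor locally at frame-rate-independent rates, while Fire spawns BP_Rocket at the Arrow's transform.
; MoveForward and some older movement and propeller nodes remain but never run.
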(event `self.ReceiveTick`
  (params (DeltaSeconds :type "Float (single-precision)"))
  (`|ExecutionSequence`
    (:`then_0`
      (`self.AddMovementInput` (`self.GetActorForwardVector`))
      (`KismetSystemLibrary.Delay` 3.0))
    (:`then_1`
      (`self.RotateComponent` (`self.PropellerL`))
      (`self.RotateComponent` (`self.PropellerR`)))))

(event `InputAxis|Pitch`
  (params (AxisValue :type "Float (single-precision)"))
  (`self.K2_AddActorLocalRotation` (`KismetMathLibrary.MakeRotator` 0.0 (* AxisValue (`GameplayStatics.GetWorldDeltaSeconds`) 60.0))))

(event `InputAxis|Roll`
  (params (AxisValue :type "Float (single-precision)"))
  (`self.K2_AddActorLocalRotation` (`KismetMathLibrary.MakeRotator` (* AxisValue (`GameplayStatics.GetWorldDeltaSeconds`) 60.0))))

(event `InputAction|Fire`
  (params (Key :type "Key Structure"))
  (:`Pressed`
    (`|SpawnActorFromClass` "/Game/BluePrint/BP_Rocket.BP_Rocket_C" (`SceneComponent.K2_GetComponentToWorld` (`self.Arrow`)) "Undefined" "MultiplyWithRoot" self self)))

(fn `MoveForward`
  (params (Speed :type "Float (double-precision)"))
  (`self.K2_AddActorWorldOffset` (* (`self.GetActorForwardVector`) 400.0 Speed)))

(fn `RotateComponent`
  (params (Parts :type "SceneComponent Object Reference"))
  (`SceneComponent.K2_AddLocalRotation` Parts (`KismetMathLibrary.MakeRotator` (* (`GameplayStatics.GetWorldDeltaSeconds`) (`self.RotationSpeed`))) false false))

(fn `UserConstructionScript`)